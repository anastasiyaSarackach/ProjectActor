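; BP_BlockDestractable is a block actor that shrinks a step each time another actor begins overlapping it.
; BeginPlay caches the Cube component's world scale and derives a fixed step of 5% of it.
; Each overlap subtracts that step and applies the result as the actor's scale, with no lower clamp or destroy call.
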(event EventBeginPlay
  (|CallParentFunction)
  (bind _output_get (Variables|Default|SetvectorScale (Transformation|GetWorldScale (Variables|Default|GetCube))))
  (Variables|Default|SetvectorDeltaScale (* _output_get "0.050000,0.050000,0.050000")))

(event Collision|EventActorBeginOverlap
  (params (OtherActor :type Actor%20Object%20Reference))
  (|CallParentFunction OtherActor)
  (bind _output_get (Variables|Default|SetvectorScale (- (Variables|Default|GetvectorScale) (Variables|Default|GetvectorDeltaScale))))
  (Transformation|SetActorScale3D _output_get))

(event EventTick
  (params (DeltaSeconds :type Float%20%28single-precision%29))
  (|CallParentFunction DeltaSeconds) ; This node is disabled and will not be called.\nDrag off pins to build functionality.
)

(fn ConstructionScript
  (|CallParentFunction))