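; BP_bonus is a moving pickup that spawns an extra Bp_ballarcade when it overlaps a BP_Pawn.
; Each tick it moves with a swept world offset of Direction times Speed squared, without scaling by delta time.
; On overlap it spawns the ball at the pawn's location minus NewDirection, then destroys itself.
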(event EventBeginPlay)

(event Collision|EventActorBeginOverlap
  (params (OtherActor :type Actor%20Object%20Reference))
  (bind _asbp_pawn (Utilities|Casting|CastToBP_Pawn OtherActor))
  (Game|SpawnActorfromClass "/Game/Work8/bp_ballarcade.bp_ballarcade_C" (Math|Conversions|ToTransform(Vector) (- (Transformation|GetActorLocation _asbp_pawn) (Variables|Default|GetnewDirection))) "Undefined" 0 0)
  (Actor|DestroyActor))

(event EventTick
  (params (DeltaSeconds :type Float%20%28single-precision%29))
  (bind _speed (Variables|Default|Getspeed))
  (Transformation|AddActorWorldOffset (* (* (Variables|Default|Getdirection) _speed) _speed) true))

(fn ConstructionScript)