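; BP_Blox lays out a grid of blocks for what appears to be an arcade ball-and-brick game.
; On BeginPlay, nested loops over X and Y call SpawnBlock to spawn Mjk actors at padded, offset positions.
; Its Hit event destroys its own struck component when bp_ballarcade is the other actor, and any overlap decrements NewVar0.
; An unconnected construction-script loop that would build the grid from static mesh components never runs.
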(event EventBeginPlay
  (for _index (range 0 (Variables|Default|Getx))
    (for _index_2 (range 0 (Variables|Default|Gety))
      (CallFunction|SpawnBlock (Math|Transform|MakeTransform (Math|Vector|MakeVector (+ (Math|Conversions|ToFloat(Integer) (* _index (Variables|Default|GetPadding))) (Variables|Default|Getoffset_x)) (+ (Math|Conversions|ToFloat(Integer) (* _index_2 (Variables|Default|GetPadding))) (Variables|Default|Getoffset_y)) 1e+02))))))

(event Collision|EventActorBeginOverlap
  (params (OtherActor :type Actor%20Object%20Reference))
  (Math|Integer|DecrementInt (Variables|Default|GetNewVar_0)))

(event EventTick
  (params (DeltaSeconds :type Float%20%28single-precision%29)))

(event Collision|EventHit
  (params (MyComp :type Primitive%20Component%20Object%20Reference) (Other :type Actor%20Object%20Reference) (OtherComp :type Primitive%20Component%20Object%20Reference) (bSelfMoved :type Boolean) (HitLocation :type Vector :default "0, 0, 0") (HitNormal :type Vector :default "0, 0, 0") (NormalImpulse :type Vector :default "0, 0, 0") (Hit :type Hit%20Result%20Structure%20%28by%20ref%29))
  (Utilities|Casting|CastTobp_ballarcade Other)
  (Components|DestroyComponent MyComp))

(fn ConstructionScript)

(fn SpawnBlock
  (params (SpawnTransform :type Transform))
  (bind _returnvalue (Game|SpawnActorfromClass "/Game/Work8/mjk.mjk_C" SpawnTransform "Undefined" 0 0))
  (return 0 _returnvalue))