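; Ball actor that travels in a straight line, bounces off whatever blocks it, and destroys itself when it overlaps a KillZVolume.
; Tick moves it manually with a swept world offset along Direction scaled by Speed and delta time, without physics simulation.
; On a blocking hit it reflects Direction about the hit normal and cuts Speed by a tenth, provided Speed is at or above MinSpeed.
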(event EventBeginPlay)

(event Collision|EventActorBeginOverlap
  (params (OtherActor :type Actor%20Object%20Reference))
  (Utilities|Casting|CastToKillZVolume OtherActor)
  (Actor|DestroyActor))

(event EventTick
  (params (DeltaSeconds :type Float%20%28single-precision%29))
  (bind _sweephitresult (Transformation|AddActorWorldOffset (* (* (Variables|Default|Getdirection) (Variables|Default|GetSpeed)) DeltaSeconds) true))
  (if (.bBlockingHit (Collision|BreakHitResult _sweephitresult))
    (Variables|Default|Setdirection (Math|Vector|GetReflectionVector (Variables|Default|Getdirection) (.Normal (Collision|BreakHitResult _sweephitresult))))
    (Math|Float|CompareFloat (Variables|Default|GetSpeed) (Variables|Default|GetminSpeed)
      (:>
        _)
      (:==
        _))
    (Variables|Default|SetSpeed (- (Variables|Default|GetSpeed) (* (Variables|Default|GetSpeed) 0.1)))))

(fn ConstructionScript)